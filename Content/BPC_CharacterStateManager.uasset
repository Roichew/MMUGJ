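; Character state component that tracks whether the player is hidden by crouching inside a bush.
; Every Tick it gets the player reference through a message call and treats one CurrentState enum value as crouching.
; It passes that result and its InsideBush flag to UpdateCharacterHiddenState, which sets IsHidden true only when both hold.
; InsideBush is only read here, never set.
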(event EventTick
  (params (DeltaSeconds :type Float%20%28single-precision%29))
  (bind _player (Class|BPIPlayerRef|GetPlayerRef(Message) self))
  (CallFunction|UpdateCharacterHiddenState (Variables|Default|GetInsideBush?) (Utilities|Enum|Equal(Enum) (Variables|/Game/ThirdPerson/Blueprints/BP_ThirdPersonCharacter.BP_ThirdPersonCharacter_C|GetCurrentState _player) "NewEnumerator1")))

(fn UpdateCharacterHiddenState
  (params (InsideBush? :type Boolean) (IsCrouching? :type Boolean))
  (if (and InsideBush? IsCrouching?)
    (Variables|Default|SetIsHidden? true)
    (else
      (Variables|Default|SetIsHidden? false))))