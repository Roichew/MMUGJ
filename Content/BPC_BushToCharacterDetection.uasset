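; Bush Blueprint that fades its dithering effect when the third-person character enters or leaves its box trigger.
; Overlap plays the Dithering timeline, which drives the Bush's "Dithering" float variable; end overlap reverses it from the end through UnDither.
; Helper functions set InsideBush and IsHidden on the player's StateManager, but their calls are disconnected, so only the visual effect runs.
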(event OnComponentBeginOverlap(Box)
  (params (OverlappedComponent :type Primitive%20Component%20Object%20Reference) (OtherActor :type Actor%20Object%20Reference) (OtherComp :type Primitive%20Component%20Object%20Reference) (OtherBodyIndex :type Integer) (bFromSweep :type Boolean) (SweepResult :type Hit%20Result%20Structure%20%28by%20ref%29))
  (bind _asbp_third_person_character (Utilities|Casting|CastToBP_ThirdPersonCharacter OtherActor))
  (Utilities|IsValid _asbp_third_person_character
    (:Is%20Valid
      (bind _dithering_time (Timeline|Dithering PlayFromStart)
        (:Update
          (Niagara|SetNiagaraVariable(Float) (Variables|Default|GetBush) "Dithering" _dithering_time))))))

(event OnComponentEndOverlap(Box)
  (params (OverlappedComponent :type Primitive%20Component%20Object%20Reference) (OtherActor :type Actor%20Object%20Reference) (OtherComp :type Primitive%20Component%20Object%20Reference) (OtherBodyIndex :type Integer))
  (bind _asbp_third_person_character (Utilities|Casting|CastToBP_ThirdPersonCharacter OtherActor))
  (Utilities|IsValid _asbp_third_person_character
    (:Is%20Valid
      (CallFunction|UnDither))))

(event Custom|UnDither
  (bind _dithering_time (Timeline|Dithering ReverseFromEnd)
    (:Update
      (Niagara|SetNiagaraVariable(Float) (Variables|Default|GetBush) "Dithering" _dithering_time))))

(event EventBeginPlay)

(fn ConstructionScript)

(fn SetinBushState
  (params (InsideBush? :type Boolean) (StateManager :type BPC%20Character%20State%20Manager%20Object%20Reference))
  (Utilities|IsValid StateManager
    (:Is%20Valid
      (Variables|/Game/BPC_CharacterStateManager.BPC_CharacterStateManager_C|SetInsideBush? StateManager InsideBush?))))

(fn SetCharacterIsHidden
  (params (StateManager :type BPC%20Character%20State%20Manager%20Object%20Reference) (CurrentState :type BPE_CharacterState%20Enum :default "NewEnumerator0"))
  (Utilities|IsValid StateManager
    (:Is%20Valid
      (Variables|/Game/BPC_CharacterStateManager.BPC_CharacterStateManager_C|SetIsHidden? StateManager (Utilities|Enum|Equal(Enum) CurrentState "NewEnumerator1")))))