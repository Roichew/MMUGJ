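; BP_E_Base is a base enemy AI character that kills the third-person player character when it overlaps the enemy's sphere.
; Chase plays a montage slot with none assigned and broadcasts OnAttackEnd when it ends, Investigate plays a sniff montage, and Attack only prints.
; Helper functions return patrol routes and switch walk or sprint speed, while the AI controller and enemy reference getters return nothing.
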(event OnComponentBeginOverlap(Sphere)
  (params (OverlappedComponent :type Primitive%20Component%20Object%20Reference) (OtherActor :type Actor%20Object%20Reference) (OtherComp :type Primitive%20Component%20Object%20Reference) (OtherBodyIndex :type Integer) (bFromSweep :type Boolean) (SweepResult :type Hit%20Result%20Structure%20%28by%20ref%29))
  (bind _asbp_third_person_character (Utilities|Casting|CastToBP_ThirdPersonCharacter OtherActor))
  (Utilities|IsValid _asbp_third_person_character
    (:Is%20Valid
      (Default|Death _asbp_third_person_character))))

(event Custom|Attack
  (Development|PrintString "Attack"))

(event Custom|Chase
  (Animation|Montage|PlayMontage (Variables|Character|GetMesh) 0
    (:OnCompleted
      _)
    (:OnInterrupted
      _))
  (Default|CallOnAttackEnd))

(event Custom|Investigate
  (Animation|Montage|PlayMontage (Variables|Character|GetMesh) "/Game/Animation/Wolf/AM_Sniff.AM_Sniff"))

(fn ConstructionScript)

(fn GetAICRef
  (return 0))

(fn GetEnemyRef
  (return 0 0))

(fn GetPatrolPoints
  (return (Variables|Default|GetPatrolRoutes)))

(fn SetMovementSpeed
  (params (Speed :type E_Speed%20Enum :default "NewEnumerator0"))
  (bind _output_get (Variables|/Script/Engine.CharacterMovementComponent|SetMaxWalkSpeed (Variables|Character|GetCharacterMovement) (Utilities|Select :Index Speed :NewEnumerator0 1e+02 :NewEnumerator1 3e+02)))
  (return _output_get))